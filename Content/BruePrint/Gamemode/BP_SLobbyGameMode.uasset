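; Lobby game mode that starts play on BeginPlay, restarting the player once and spawning an enemy.
; BeginPlay passes through an intro cutscene event into StartGame, guarded by GameInProgress; cutscene lookup and start sound nodes are unconnected.
; StartEnemySpawn spawns a single BP_Minion at a randomly chosen BP_SpawnActor transform, without checking the lookup's Valid flag.
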(event Custom|PlayDefaultIntroCutscene
  (CallFunction|StartGame))

(event Custom|StartGame
  (if (not (Variables|Default|GetbGameInProgress))
    (Variables|Default|SetbGameInProgress true)
    (Class|GameModeBase|RestartPlayer (CallFunction|GetPlayerControllerBP))
    (CallFunction|StartEnemySpawn)))

(event EventBeginPlay
  (CallFunction|PlayDefaultIntroCutscene))

(event EventTick
  (params (DeltaSeconds :type Float%20%28single-precision%29)))

(event Custom|StartEnemySpawn
  (Game|SpawnActorfromClass "/Game/BruePrint/Character/Enemy/BP_Minion.BP_Minion_C" (.Transform (CallFunction|GetRandomSpawnPoint)) "AdjustIfPossibleButAlwaysSpawn" "MultiplyWithRoot" 0 0))

(fn ConstructionScript)

(fn GetRandomSpawnPoint
  ;[1 1 1] 등록된 모든 엑터를 가져와 그 중 랜덤하게 위치 가져오는 함수
  (bind _outactors (Actor|GetAllActorsOfClass "/Game/BruePrint/BP/BP_SpawnActor.BP_SpawnActor_C"))
  (if (Utilities|Array|IsValidIndex _outactors)
    (bind _output_get (LocalVariables|SetSpawnPoint (Transformation|GetActorTransform (Utilities|Array|Get(acopy) _outactors (Math|Random|RandomIntegerinRange 0 (Utilities|Array|LastIndex _outactors))))))
    (return true _output_get)
    (else
      (return (Utilities|Array|IsValidIndex _outactors) (LocalVariables|GetSpawnPoint)))))