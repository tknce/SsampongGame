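; GA_Sprint_BP is the player's sprint Gameplay Ability, active while input is held.
; Activation applies GE_StandardSprint and a gameplay cue, then starts sprinting on SBelicaMovementComponent.
; A short-delay, net-synced loop commits cost while accelerating on the ground, but stops looping otherwise without ending the ability.
; Input release or failed cost ends the ability, removing the effect and stopping sprint.
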(event Ability|EventActivateAbility
  (Variables|Default|SetEndSprint false)
  (bind _returnvalue (Ability|ApplyGameplayEffectToOwner "/Game/BruePrint/Character/Shared/GameplayEffectTemplates/GE_StandardSprint.GE_StandardSprint_C" (Ability|GetAbilityLevel)))
  (Variables|Default|SetGESprint _returnvalue)
  (GameplayCue|AddGameplayCue :GameplayCueTag "(TagName=\"GameplayCue.Hero.Spint\")")
  (bind _assbelica_movement_component (Utilities|Casting|CastToSBelicaMovementComponent (.MovementComponent (Utilities|Struct|BreakGameplayAbilityActorInfo (Ability|GetActorInfo)))))
  (Class|SBelicaMovementComponent|StartSprinting _assbelica_movement_component)
  (Ability|Tasks|WaitInputRelease true
    (:then
      (Ability|Tasks|WaitDelay 0.05 :!label _label
        (:OnFinish
          (Ability|Tasks|WaitNetSync "BothWait"
            (:OnSync
              (bind _assbelica_movement_component_2 (Utilities|Casting|CastToSBelicaMovementComponent (.MovementComponent (Utilities|Struct|BreakGameplayAbilityActorInfo (Ability|GetActorInfo)))))
              (if (and (> (Math|Vector|VectorLength (Pawn|Components|CharacterMovement|GetCurrentAcceleration _assbelica_movement_component_2)) 0.0) (not (AI|Components|NavMovement|IsFalling _assbelica_movement_component_2)))
                (bind _returnvalue_2 (Ability|CommitAbilityCost false))
                (if _returnvalue_2
                  (if (not (Variables|Default|GetEndSprint))
                    (goto _label))
                  (else
                    (Variables|Default|SetEndSprint true :!label _label_2)
                    (Ability|EndAbility)))))))))
    (:OnRelease
      (goto _label_2))))

(event Ability|EventOnEndAbility
  (params (bWasCancelled :type Boolean))
  (Ability|RemoveGameplayEffectFromOwnerWithHandle (Variables|Default|GetGESprint))
  (bind _assbelica_movement_component (Utilities|Casting|CastToSBelicaMovementComponent (.MovementComponent (Utilities|Struct|BreakGameplayAbilityActorInfo (Ability|GetActorInfo)))))
  (Class|SBelicaMovementComponent|StopSprinting _assbelica_movement_component))