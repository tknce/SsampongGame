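; Gameplay ability that puts the Belica player character into aim-down-sights while the input is held.
; On activation it applies a gameplay effect, shortens the camera boom and starts ADS on SBelicaMovementComponent; input release ends the ability.
; On end it restores the starting boom length, stops ADS and removes effects by handle.
; Activation and end both apply GE_StandardAimDownSightRemoval, with the end instance removed immediately.
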(event Ability|EventActivateAbility
  (bind _assbelica_player_character (Utilities|Casting|CastToSBelicaPlayerCharacter (Ability|GetAvatarActorfromActorInfo)))
  (Variables|Default|SetOwningBelica _assbelica_player_character)
  (bind _returnvalue (Ability|ApplyGameplayEffectToOwner "/Game/BruePrint/Character/Shared/GameplayEffectTemplates/GE_StandardAimDownSightRemoval.GE_StandardAimDownSightRemoval_C" (Ability|GetAbilityLevel)))
  (Variables|Default|SetGEAimDownSight _returnvalue)
  (Variables|/Script/Engine.SpringArmComponent|SetTargetArmLength (Variables|/Script/SsampongGame.SBelicaPlayerCharacter|GetCameraBoom (Variables|Default|GetOwningBelica)) 1e+02)
  (bind _assbelica_movement_component (Utilities|Casting|CastToSBelicaMovementComponent (.MovementComponent (Utilities|Struct|BreakGameplayAbilityActorInfo (Ability|GetActorInfo)))))
  (Class|SBelicaMovementComponent|StartAimDownSights _assbelica_movement_component)
  (Ability|Tasks|WaitInputRelease false
    (:OnRelease
      (Ability|EndAbility))))

(event Ability|EventOnEndAbility
  (params (bWasCancelled :type Boolean))
  (bind _owningbelica (Variables|Default|GetOwningBelica))
  (bind _returnvalue (Ability|ApplyGameplayEffectToOwner "/Game/BruePrint/Character/Shared/GameplayEffectTemplates/GE_StandardAimDownSightRemoval.GE_StandardAimDownSightRemoval_C" (Ability|GetAbilityLevel)))
  (Variables|Default|SetGEAimDownSightRemoval _returnvalue)
  (Ability|RemoveGameplayEffectFromOwnerWithHandle (Variables|Default|GetGEAimDownSight))
  (Ability|RemoveGameplayEffectFromOwnerWithHandle (Variables|Default|GetGEAimDownSightRemoval))
  (Variables|/Script/Engine.SpringArmComponent|SetTargetArmLength (Variables|/Script/SsampongGame.SBelicaPlayerCharacter|GetCameraBoom _owningbelica) (Variables|/Script/SsampongGame.SBelicaPlayerCharacter|GetStartingCameraBoomArmLength _owningbelica))
  (bind _assbelica_movement_component (Utilities|Casting|CastToSBelicaMovementComponent (.MovementComponent (Utilities|Struct|BreakGameplayAbilityActorInfo (Ability|GetActorInfo)))))
  (Class|SBelicaMovementComponent|StopAimDownSights _assbelica_movement_component))