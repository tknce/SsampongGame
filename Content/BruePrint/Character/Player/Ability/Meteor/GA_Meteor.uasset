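; Meteor gameplay ability for the Belica player character that drops a damaging rock on a player-chosen location.
; On activation it shows the confirm/cancel prompt, raises the camera boom and runs WaitTargetData until the player confirms or cancels.
; After a successful commit, only the authority spawns the rock above the target, handing it a SetByCaller damage effect spec.
; Ending the ability restores the camera and hides the prompt.
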(event Ability|EventActivateAbility
  (bind _returnvalue (Class|GameplayAbility|MakeTargetLocationInfofromOwnerActor))
  (bind (_locationtype _literaltransform _sourceactor _sourcecomponent _sourceability _sourcesocketname) (Utilities|Struct|BreakGameplayAbilityTargetingLocationInfo _returnvalue))
  (bind _assbelica_player_character (Utilities|Casting|CastToSBelicaPlayerCharacter (Ability|GetAvatarActorfromActorInfo)))
  (Variables|Default|SetOwningBelica _assbelica_player_character)
  (bind _assbelica_player_state (Utilities|Casting|CastToSBelicaPlayerState (Ability|GetOwningActorfromActorInfo)))
  (Class|SBelicaPlayerState|ShowAbilityConfirmCancelText _assbelica_player_state true)
  (Transformation|SetRelativeLocation (Variables|/Script/SsampongGame.SBelicaPlayerCharacter|GetCameraBoom (Variables|Default|GetOwningBelica)) (Math|Vector|MakeVector (.x (Variables|/Script/SsampongGame.SBelicaPlayerCharacter|GetStartingCameraBoomLocation (Variables|Default|GetOwningBelica))) (.y (Variables|/Script/SsampongGame.SBelicaPlayerCharacter|GetStartingCameraBoomLocation (Variables|Default|GetOwningBelica))) (+ (.z (Variables|/Script/SsampongGame.SBelicaPlayerCharacter|GetStartingCameraBoomLocation (Variables|Default|GetOwningBelica))) 1e+02)) false false)
  (bind _data (|WaitTargetData :ConfirmationType "UserConfirmed" :Class (Variables|Default|GetTargetActorClass) :MaxRange (Variables|Default|GetRange) :TraceProfile "(Name=\"TargetActorGroundLocation\")" :StartLocation (Utilities|Struct|MakeGameplayAbilityTargetingLocationInfo _locationtype (Math|Transform|MakeTransform (+ (* (Transformation|GetActorForwardVector (Variables|Default|GetOwningBelica)) 2e+02) (.location _literaltransform)) (.rotation _literaltransform) (.scale _literaltransform)) _sourceactor _sourcecomponent _sourceability _sourcesocketname) :ReticleClass 0)
    (:ValidData
      (bind _returnvalue_2 (Ability|CommitAbility))
      (if _returnvalue_2
        (if (Ability|HasAuthority (Variables|Default|GetOwningBelica))
          (bind _returnvalue_3 (Ability|GameplayEffect|AssignTagSetbyCallerMagnitude (Ability|MakeOutgoingGameplayEffectSpec (Variables|Default|GetDamegeGameplayEffectClass) (Math|Conversions|ToFloat(Integer) (Ability|GetAbilityLevel))) "(TagName=\"Data.Damage\")" (Variables|Default|GetDamage)))
          (Game|SpawnActorfromClass (Variables|Default|GetRockClass) (Math|Transform|MakeTransform (+ (.Location (Collision|BreakHitResult (Ability|TargetData|GetHitResultfromTargetData _data))) "0.000000,0.000000,1000.000000") "0, 0, 0" "1.000000,1.000000,1.000000") "AlwaysSpawn" "MultiplyWithRoot" (Variables|Default|GetOwningBelica) 0.0 _returnvalue_3 (Variables|Default|GetOwningBelica))
          (Ability|EndAbility)
          (else
            (Ability|EndAbility)))
        (else
          (Ability|CancelAbility :!label _label))))
    (:Cancelled
      (goto _label))))

(event Ability|EventOnEndAbility
  (params (bWasCancelled :type Boolean))
  (bind _owningbelica (Variables|Default|GetOwningBelica))
  (Transformation|SetRelativeLocation (Variables|/Script/SsampongGame.SBelicaPlayerCharacter|GetCameraBoom _owningbelica) (Variables|/Script/SsampongGame.SBelicaPlayerCharacter|GetStartingCameraBoomLocation _owningbelica) false false)
  (bind _assbelica_player_state (Utilities|Casting|CastToSBelicaPlayerState (Ability|GetOwningActorfromActorInfo)))
  (Class|SBelicaPlayerState|ShowAbilityConfirmCancelText _assbelica_player_state false))