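; BP_Meteor is a meteor ability actor that damages and stuns characters around it when its collision sphere begins an overlap.
; On authority, it gathers overlapping SBelicaCharacter actors, skipping dead ones and its instigator.
; It applies its stored damage and stun Gameplay Effect specs through each target's Ability System Component, then destroys itself.
; A debug print names overlapped components that are neither WorldStatic nor WorldDynamic.
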(event OnComponentBeginOverlap(SphereCollision)
  (params (OverlappedComponent :type Primitive%20Component%20Object%20Reference) (OtherActor :type Actor%20Object%20Reference) (OtherComp :type Primitive%20Component%20Object%20Reference) (OtherBodyIndex :type Integer) (bFromSweep :type Boolean) (SweepResult :type Hit%20Result%20Structure%20%28by%20ref%29))
  (bind _returnvalue (Collision|GetCollisionObjectType OtherComp))
  (if (or (Utilities|Enum|Equal(Enum) _returnvalue "ECC_WorldStatic") (Utilities|Enum|Equal(Enum) _returnvalue "ECC_WorldDynamic"))
    _
    (else
      (Development|PrintString (Utilities|GetObjectName OtherComp))))
  (Networking|SwitchHasAuthority
    (:Authority
      (for _array_element (Collision|GetOverlappingActors (Variables|Default|GetSphereCollision) "/Script/SsampongGame.SBelicaCharacter" :!class /Script/Engine.PrimitiveComponent)
        (bind _assbelica_character (Utilities|Casting|CastToSBelicaCharacter _array_element))
        (if (Math|Boolean|ANDBoolean (Class|SBelicaCharacter|IsAlive _assbelica_character) (not (== _assbelica_character (Game|GetInstigator))) (Utilities|IsValid (Ability|GetAbilitySystemComponent _assbelica_character)))
          (GameplayEffects|ApplyGameplayEffectSpecToSelf (Ability|GetAbilitySystemComponent _assbelica_character) (Variables|Default|GetDamageEffectSpecHandle))
          (GameplayEffects|ApplyGameplayEffectSpecToSelf (Ability|GetAbilitySystemComponent _assbelica_character) (Variables|Default|GetStunEffectSpecHandle)))))
    (:Remote
      _))
  (Actor|DestroyActor))

(event EventBeginPlay)

(event EventTick
  (params (DeltaSeconds :type Float%20%28single-precision%29)))

(fn ConstructionScript)