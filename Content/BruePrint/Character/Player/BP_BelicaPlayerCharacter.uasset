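; Belica player character Blueprint that sketches a left-click melee-style combo attack, currently left unwired.
; A raw mouse key starts the attack or buffers a click; ComboAttackSave replays a buffered click into the ComboCount switch, and ResetCombo clears the state.
; The switch has no connected branches, the three attack montages are disconnected, and ComboCount never increments.
; Tick only casts to SBelicaPlayerState; its health and mana reads are unused.
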(event Custom|ResetCombo
  ;[1 1 1] Combo System Setup.
  (Variables|Default|SetComboCount 0)
  (Variables|Default|SetSaveAttack false)
  (Variables|Default|SetIsAttacking false))

(event Custom|ComboAttackSave
  ;[1 1 1] Combo System Setup.
  (if (Variables|Default|GetSaveAttack)
    (Variables|Default|SetSaveAttack false)
    (switch int (Variables|Default|GetComboCount))))

(event EventBeginPlay)

(event Collision|EventActorBeginOverlap
  (params (OtherActor :type Actor%20Object%20Reference)))

(event EventTick
  (params (DeltaSeconds :type Float%20%28single-precision%29))
  (bind _assbelica_player_state (Utilities|Casting|CastToSBelicaPlayerState (Game|GetPlayerState 0))))

(event Input|MouseEvents|LeftMouseButton
  (params (Key :type Key%20Structure))
  ;[1 1 1] Simple attack setup. Intentionally not using inputs so that this will "just work" with the 3rd Person Template. If you were doing this for real, you would set up a proper input.
  (:Pressed
    ;[1 1 1] Combo System Setup.
    (if (Variables|Default|GetIsAttacking)
      (Variables|Default|SetSaveAttack true)
      (else
        (Variables|Default|SetIsAttacking true)
        (switch int (Variables|Default|GetComboCount))))))

(fn ConstructionScript)