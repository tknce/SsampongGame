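; Enemy attack projectile that delivers a Gameplay Ability System damage effect to SBelicaCharacter.
; Its lifespan is derived from Range and initial speed, capping travel distance.
; Overlaps ignore the instigator; on authority, a pawn line trace toward the character supplies a hit result for the effect context before DamageEffectSpecHandle is applied.
; It destroys itself after applying damage, on overlapping other actors, or on any non-instigator overlap on remotes.
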(event OnComponentBeginOverlap(Collision)
  (params (OverlappedComponent :type Primitive%20Component%20Object%20Reference) (OtherActor :type Actor%20Object%20Reference) (OtherComp :type Primitive%20Component%20Object%20Reference) (OtherBodyIndex :type Integer) (bFromSweep :type Boolean) (SweepResult :type Hit%20Result%20Structure%20%28by%20ref%29))
  (if (!= OtherActor (Game|GetInstigator))
    (Networking|SwitchHasAuthority
      (:Authority
        (bind _assbelica_character (Utilities|Casting|CastToSBelicaCharacter OtherActor)
          (:then
            (if (Utilities|IsValid (Ability|GetAbilitySystemComponent _assbelica_character))
              (bind _outhits (Class|KismetSystemLibrary|LineTraceMultiforObjects (Transformation|GetActorLocation) (Transformation|GetActorLocation _assbelica_character) (Utilities|Array|MakeArray "ObjectTypeQuery3") false 0 "None" true))
              (bind _array_element (Utilities|Array|ForEachLoopwithBreak _outhits :!label _label)
                (:LoopBody
                  (if (== _assbelica_character (.HitActor (Collision|BreakHitResult _array_element)))
                    (Variables|Default|SetFinalHit _array_element)
                    (goto _label Break)))
                (:Completed
                  (bind _returnvalue (Class|AbilitySystemBlueprintLibrary|GetEffectContext (Variables|Default|GetDamageEffectSpecHandle)))
                  (Class|AbilitySystemBlueprintLibrary|EffectContextAddHitResult _returnvalue (Variables|Default|GetFinalHit) false)
                  (GameplayEffects|ApplyGameplayEffectSpecToSelf (Ability|GetAbilitySystemComponent _assbelica_character) (Variables|Default|GetDamageEffectSpecHandle))
                  (Actor|DestroyActor)))))
          (:CastFailed
            (Actor|DestroyActor :!label _label_2))))
      (:Remote
        (goto _label_2)))))

(event OnComponentBeginOverlap(Sphere)
  (params (OverlappedComponent :type Primitive%20Component%20Object%20Reference) (OtherActor :type Actor%20Object%20Reference) (OtherComp :type Primitive%20Component%20Object%20Reference) (OtherBodyIndex :type Integer) (bFromSweep :type Boolean) (SweepResult :type Hit%20Result%20Structure%20%28by%20ref%29))
  (if (!= (stale OnComponentBeginOverlap(Collision) OtherActor) (Game|GetInstigator))
    (Networking|SwitchHasAuthority
      (:Authority
        (bind _assbelica_character (Utilities|Casting|CastToSBelicaCharacter (stale OnComponentBeginOverlap(Collision) OtherActor))
          (:then
            (if (Utilities|IsValid (Ability|GetAbilitySystemComponent _assbelica_character))
              (bind _outhits (Class|KismetSystemLibrary|LineTraceMultiforObjects (Transformation|GetActorLocation) (Transformation|GetActorLocation _assbelica_character) (Utilities|Array|MakeArray "ObjectTypeQuery3") false 0 "None" true))
              (bind _array_element (Utilities|Array|ForEachLoopwithBreak _outhits :!label _label)
                (:LoopBody
                  (if (== _assbelica_character (.HitActor (Collision|BreakHitResult _array_element)))
                    (Variables|Default|SetFinalHit _array_element)
                    (goto _label Break)))
                (:Completed
                  (bind _returnvalue (Class|AbilitySystemBlueprintLibrary|GetEffectContext (Variables|Default|GetDamageEffectSpecHandle)))
                  (Class|AbilitySystemBlueprintLibrary|EffectContextAddHitResult _returnvalue (Variables|Default|GetFinalHit) false)
                  (GameplayEffects|ApplyGameplayEffectSpecToSelf (Ability|GetAbilitySystemComponent _assbelica_character) (Variables|Default|GetDamageEffectSpecHandle))
                  (Actor|DestroyActor)))))
          (:CastFailed
            (Actor|DestroyActor :!label _label_2))))
      (:Remote
        (goto _label_2)))))

(event EventBeginPlay
  (Actor|SetLifeSpan (/ (Variables|Default|GetRange) (Variables|/Script/Engine.ProjectileMovementComponent|GetInitialSpeed (Variables|Default|GetProjectileMovement)))))

(fn ConstructionScript)