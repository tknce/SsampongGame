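; BP_WeaponActor is a weapon actor that detects hits during attack windows and reports them to its wielder's abilities.
; BeginWeaponAttack stores the event tag and enables capsule query collision; EndWeaponAttack disables it after a short delay.
; Overlaps with actors of a different class than the instigator send that Gameplay Event to the instigator, gated by a DoOnce.
; Hits can trigger a count-limited hit pause through brief global time dilation.
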(event Custom|Event%20BeginWeaponAttack
  (params (Event%20Tag :type Gameplay%20Tag%20Structure) (Attack%20Delay%20Time :type Float%20%28double-precision%29) (Attack%20Delay%20Count :type Integer))
  (Variables|WeaponDeaults|SetAttackEventTag Event%20Tag)
  (Variables|WeaponDeaults|SetAttackDelayTime Attack%20Delay%20Time)
  (Variables|WeaponDeaults|SetAttackDelayCount Attack%20Delay%20Count)
  (Variables|WeaponDeaults|SetIsAttacking true)
  (Collision|SetCollisionEnabled (Variables|Default|GetCapsuleCollision) "QueryOnly"))

(event Custom|Event%20EndWeaponAttack
  (Utilities|FlowControl|Delay 0.2)
  (Variables|WeaponDeaults|SetIsAttacking false)
  (Collision|SetCollisionEnabled (Variables|Default|GetCapsuleCollision) "NoCollision"))

(event Custom|HitPause
  (if (and (> (Variables|WeaponDeaults|GetAttackDelayCount) 0) (Variables|WeaponDeaults|GetEnableAttackDelay))
    (Math|Integer|DecrementInt (Variables|WeaponDeaults|GetAttackDelayCount)
      (:%20%20
        (Utilities|FlowControl|Delay 0.1)
        (Utilities|Time|SetGlobalTimeDilation 0.1)
        (Utilities|FlowControl|Delay 0.01)
        (Utilities|Time|SetGlobalTimeDilation 1.0)))))

(event Collision|EventActorBeginOverlap
  (params (OtherActor :type Actor%20Object%20Reference))
  (bind _returnvalue (Game|GetInstigator))
  (if (and (!= (Utilities|GetClass OtherActor) (Utilities|GetClass (Game|GetInstigator))) (Variables|WeaponDeaults|GetIsAttacking)) ; 자기 자신이 피격되지 않을 때
    (Utilities|FlowControl|DoOnce false
      (:Completed
        (Ability|SendGameplayEventtoActor _returnvalue (Variables|WeaponDeaults|GetAttackEventTag) (Utilities|Struct|MakeGameplayEventData "" _returnvalue OtherActor)) ; 적중하면 어빌리티로 보냄
        (CallFunction|HitPause)))))

(event EventBeginPlay
  (Collision|IgnoreActorwhenMoving (Variables|Default|GetCapsuleCollision) 0 false))

(event Collision|EventActorEndOverlap
  (params (OtherActor :type Actor%20Object%20Reference))
  (bind _returnvalue (Game|GetInstigator))
  (Utilities|FlowControl|Delay 0.2)
  (Utilities|FlowControl|DoOnce false) ; enters at Reset
)

(fn ConstructionScript)