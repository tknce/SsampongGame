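; BP_BSFunctionLibrary is a Blueprint function library of typed getters for core gameplay objects.
; It casts a character's mesh anim instance to the Belica player AnimBlueprint and the current game mode to BP_SLobbyGameMode.
; The controller getter prefers the valid reference stored on that game mode, falling back to casting player controller 0 to BP_PlayerController.
; GetPlayerCharacterBP is an empty stub.
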(fn GetPlayerAnimBP
  (params (Character :type Character%20Object%20Reference))
  (bind _asabp_belica_player_anim_blueprint (Utilities|Casting|CastToABP_BelicaPlayer_AnimBlueprint (Components|SkeletalMesh|GetAnimInstance (Variables|/Script/Engine.Character|GetMesh Character))))
  (return _asabp_belica_player_anim_blueprint))

(fn GetPlayerCharacterBP
  (return 0))

(fn GetPlayerControllerBP
  (if (Utilities|IsValid (Variables|/Game/BruePrint/Gamemode/BP_SLobbyGameMode.BP_SLobbyGameMode_C|GetPlayerController (CallFunction|GetGameModeBP)))
    (return (Variables|/Game/BruePrint/Gamemode/BP_SLobbyGameMode.BP_SLobbyGameMode_C|GetPlayerController (CallFunction|GetGameModeBP)))
    (else
      (bind _asbp_player_controller (Utilities|Casting|CastToBP_PlayerController (Game|GetPlayerController 0)))
      (return _asbp_player_controller))))

(fn GetGameModeBP
  (bind _asbp_slobby_game_mode (Utilities|Casting|CastToBP_SLobbyGameMode (Game|GetGameMode))
    (:then
      _)
    (:CastFailed
      _))
  (return _asbp_slobby_game_mode))